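; BP_Tiles holds the triangular board of 28 sprite tiles for a Q*bert game and changes the sprite of the tile at a given position.
; On BeginPlay it adds the tiles to TilesRef row by row, from seven tiles down to one.
; SetTileSprite sums the shrinking row lengths below Position.Z, adds Position.X to get the flat array index, and sets that tile to the NextTile sprite.
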(event `self.ReceiveBeginPlay`
  (`self.AddTileToTilesArray` (`self.Tile00`))
  (`self.AddTileToTilesArray` (`self.Tile01`))
  (`self.AddTileToTilesArray` (`self.Tile02`))
  (`self.AddTileToTilesArray` (`self.Tile03`))
  (`self.AddTileToTilesArray` (`self.Tile04`))
  (`self.AddTileToTilesArray` (`self.Tile05`))
  (`self.AddTileToTilesArray` (`self.Tile06`))
  (`self.AddTileToTilesArray` (`self.Tile10`))
  (`self.AddTileToTilesArray` (`self.Tile11`))
  (`self.AddTileToTilesArray` (`self.Tile12`))
  (`self.AddTileToTilesArray` (`self.Tile13`))
  (`self.AddTileToTilesArray` (`self.Tile14`))
  (`self.AddTileToTilesArray` (`self.Tile15`))
  (`self.AddTileToTilesArray` (`self.Tile20`))
  (`self.AddTileToTilesArray` (`self.Tile21`))
  (`self.AddTileToTilesArray` (`self.Tile22`))
  (`self.AddTileToTilesArray` (`self.Tile23`))
  (`self.AddTileToTilesArray` (`self.Tile24`))
  (`self.AddTileToTilesArray` (`self.Tile30`))
  (`self.AddTileToTilesArray` (`self.Tile31`))
  (`self.AddTileToTilesArray` (`self.Tile32`))
  (`self.AddTileToTilesArray` (`self.Tile33`))
  (`self.AddTileToTilesArray` (`self.Tile40`))
  (`self.AddTileToTilesArray` (`self.Tile41`))
  (`self.AddTileToTilesArray` (`self.Tile42`))
  (`self.AddTileToTilesArray` (`self.Tile50`))
  (`self.AddTileToTilesArray` (`self.Tile51`))
  (`self.AddTileToTilesArray` (`self.Tile60`)))

(fn `AddTileToTilesArray`
  (params (NewParam :type "PaperSpriteComponent Object Reference"))
  (`KismetArrayLibrary.Array_Add` (`self.TilesRef`) NewParam))

(fn `SetTileSprite`
  (params (Position :type "Vector Structure"))
  (locals (Value :type Integer))
  ;[1 1 1] in:(Z=1) out:(7+X)     in:(Z=2) out:(13+X)     in:(Z=3) out(18+X)
  (for _index (range (+ (`KismetMathLibrary.FTrunc` (- (.z Position) 1.0)) 1))
    (bind _output_get (set `local.Value` (+ (`local.Value`) (- 7 _index)))))
  (`PaperSpriteComponent.SetSprite` (`|GetArrayItem` (`self.TilesRef`) (+ _output_get (`KismetMathLibrary.FTrunc` (.x Position)))) (`self.NextTile`)))

(fn `UserConstructionScript`)